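; BP_Ghost is a maze-chaser style enemy that kills the VRPawn on overlap, or dies itself while powered down.
; Each tick it moves along one of four axis-aligned directions selected by CurrentDirection, with no turning logic in this Blueprint.
; PoweredDown makes it vulnerable until a short timer calls PoweredUp.
; Its Die function respawns it by teleporting to a fixed location and resetting its direction.
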(event Custom|PoweredDown
  (Variables|Default|SetIsPoweredDown true)
  (bind _returnvalue (Utilities|Time|SetTimerbyEvent (delegate Custom|PoweredUp) 2.0))
  (Variables|Default|SetPowerDownTimer _returnvalue))

(event Custom|PoweredUp
  (Variables|Default|SetIsPoweredDown false)
  (Utilities|Time|ClearandInvalidateTimerbyHandle (Variables|Default|GetPowerDownTimer)))

(event Collision|EventActorBeginOverlap
  (params (OtherActor :type Actor%20Object%20Reference))
  (if (== "/Game/VRTemplate/Blueprints/VRPawn.VRPawn" OtherActor)
    (if (Variables|Default|GetIsPoweredDown)
      (CallFunction|Die)
      (else
        (bind _asvrpawn (Utilities|Casting|CastToVRPawn OtherActor))
        (Default|Die _asvrpawn)))))

(event EventTick
  (params (DeltaSeconds :type Float%20%28single-precision%29))
  (Pawn|Input|AddMovementInput (Math|Conversions|ToVector(Vector2D) (Utilities|Select :Index (Variables|Default|GetCurrentDirection) :Option%200 "(X=0.000000,Y=1.000000)" :Option%201 "(X=1.000000,Y=0.000000)" :Option%202 "(X=0.000000,Y=-1.000000)" :Option%203 "(X=-1.000000,Y=0.000000)")) 2.0 false))

(fn ConstructionScript)

(fn Die
  (Transformation|SetActorLocationAndRotation "0.000000,0.000000,70.000000" "0, 0, 0")
  (Variables|Default|SetCurrentDirection 1))