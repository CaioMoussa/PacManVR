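; BP_Consumable is a collectible orb that the VR pawn picks up by touching it.
; On overlap with an actor of the VRPawn class, it runs Consumed and destroys itself.
; Consumed casts player pawn 0 to VRPawn, rather than using the overlapping actor, then increments its orb count and adds this item's Points value to its score.
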(event Collision|EventActorBeginOverlap
  (params (OtherActor :type Actor%20Object%20Reference))
  (if (Utilities|ClassIsChildOf (Utilities|GetClass OtherActor) "/Game/VRTemplate/Blueprints/VRPawn.VRPawn_C")
    (CallFunction|Consumed)
    (Actor|DestroyActor)))

(fn ConstructionScript)

(fn Consumed
  (bind _asvrpawn (Utilities|Casting|CastToVRPawn (Game|Player|GetPlayerPawn 0)))
  (Variables|/Game/VRTemplate/Blueprints/VRPawn.VRPawn_C|SetOrbsCollected _asvrpawn (+ 1 (Variables|/Game/VRTemplate/Blueprints/VRPawn.VRPawn_C|GetOrbsCollected _asvrpawn)))
  (Variables|/Game/VRTemplate/Blueprints/VRPawn.VRPawn_C|SetPoints _asvrpawn (+ (Variables|/Game/VRTemplate/Blueprints/VRPawn.VRPawn_C|GetPoints _asvrpawn) (Variables|Default|GetPoints))))