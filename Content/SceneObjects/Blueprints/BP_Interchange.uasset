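; BP_Interchange is a junction actor that redirects ghosts passing through it.
; On overlap with a BP_Ghost, it sets the ghost's CurrentDirection to a random entry from its PossibleDirections.
; It then sets the ghost's MaxWalkSpeed to zero and immediately to a fixed high value, with no delay between.
; An unconnected node for snapping the overlapping actor to the junction's position never runs.
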(event Collision|EventActorBeginOverlap
  (params (OtherActor :type Actor%20Object%20Reference))
  (if (Utilities|ClassIsChildOf (Utilities|GetClass OtherActor) "/Game/SceneObjects/Blueprints/BP_Ghost.BP_Ghost_C")
    (bind _asbp_ghost (Utilities|Casting|CastToBP_Ghost OtherActor))
    (Variables|/Game/SceneObjects/Blueprints/BP_Ghost.BP_Ghost_C|SetCurrentDirection _asbp_ghost (.OutItem (Utilities|Array|Random (Variables|Default|GetPossibleDirections))))
    (Variables|/Script/Engine.CharacterMovementComponent|SetMaxWalkSpeed (Variables|/Script/Engine.Character|GetCharacterMovement _asbp_ghost) 0.0)
    (Variables|/Script/Engine.CharacterMovementComponent|SetMaxWalkSpeed (Variables|/Script/Engine.Character|GetCharacterMovement _asbp_ghost) 5e+03)))

(fn ConstructionScript)